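; BP_GreatSword is a melee weapon Blueprint that deals combo-scaled damage to actors its capsule hitbox overlaps.
; The capsule's collision is off at BeginPlay and is switched on and off by the parent's OnCollision and OffCollision events.
; On overlap it asks DamageComponent for the damage of the current ComboCount and passes it to SendDamage.
; StartCombo and EndCombo extend the parent events to start and end the DamageComponent's attack.
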(event `self.ReceiveBeginPlay`
  (`parent.ReceiveBeginPlay`)
  (`PrimitiveComponent.SetCollisionEnabled` (`self.Capsule`) "NoCollision"))

(event `self.OnCollision`
  (params (CollisionType :type "/Game/Enums/ECollisionType Enum" :default "NewEnumerator0"))
  (`parent.OnCollision` CollisionType)
  (`PrimitiveComponent.SetCollisionEnabled` (`self.Capsule`) "QueryAndPhysics"))

(event `self.OffCollision`
  (`parent.OffCollision`)
  (`PrimitiveComponent.SetCollisionEnabled` (`self.Capsule`) "NoCollision"))

(event `self.Capsule.OnComponentBeginOverlap`
  (params (OverlappedComponent :type "PrimitiveComponent Object Reference") (OtherActor :type "Actor Object Reference") (OtherComp :type "PrimitiveComponent Object Reference") (OtherBodyIndex :type Integer) (bFromSweep :type Boolean) (SweepResult :type "HitResult Structure (by ref)"))
  (bind _returnvalue (`/Game/Components/DamageComponent.GetComboDamage` (`self.DamageComponent`) (`self.ComboCount`)))
  (`self.SendDamage` OtherActor _returnvalue))

(event `self.StartCombo`
  (`parent.StartCombo`)
  (`/Game/Components/DamageComponent.StartAttack` (`self.DamageComponent`)))

(event `self.EndCombo`
  (`parent.EndCombo`)
  (`/Game/Components/DamageComponent.EndAttack` (`self.DamageComponent`)))

(fn `UserConstructionScript`)