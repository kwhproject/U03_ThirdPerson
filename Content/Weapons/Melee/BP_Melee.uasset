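; Melee weapon Blueprint that runs combo attacks and passes damage to its parent class.
; BeginPlay collects data table rows matching its MeleeType, each defining a combo step's montage, play rate, section and movement permission.
; Attack starts the combo or, while CanCombo is set, queues the next step for PlayNextCombo; EndAttack resets it.
; SendDamage tracks hit actors until OffCollision clears them; OnCollision, StartCombo and EndCombo are empty.
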(event `self.ReceiveBeginPlay`
  ;[1 1 1] Read Melee Datas
  (`parent.ReceiveBeginPlay`)
  (bind _outrownames (`DataTableFunctionLibrary.GetDataTableRowNames` (`self.DataTable`)))
  (for _array_element _outrownames
    (bind _returnvalue (`|GetDataTableRow` (`self.DataTable`) _array_element)
      (:`then`
        (if (== (`.Type_16_D38C7A244F3D06C2C29C93A3A4F333F1` (break `/Game/Structs/FMelee` _returnvalue)) (`self.MeleeType`))
          (`KismetArrayLibrary.Array_Add` (`self.MeleeDatas`) _returnvalue))))))

(event `self.Attack`
  ;[1 1 1] Attack
  (`parent.Attack`)
  (if (`self.bCanCombo`)
    (set `self.bCanCombo` false)
    (set `self.bSucceedCombo` true)
    (elif (`self.CanAttack`)
      (`self.SetStateAttacking`)
      (`self.PlayComboMontage`)
      (`self.StartCombo`))))

(event `PlayNextCombo`
  ;[1 1 1] PlayNextCombo
  (if (`self.bSucceedCombo`)
    (set `self.bSucceedCombo` false)
    (`/Engine/EditorBlueprintResources/StandardMacros.IncrementInt` (`self.ComboCount`)
      (:`  `
        (`self.PlayComboMontage`)))))

(event `self.EndAttack`
  ;[1 1 1] EndAttack
  (`parent.EndAttack`)
  (`self.SetStateIdling`)
  (`self.SetMove` true)
  (set `self.ComboCount` 0)
  (`self.EndCombo`))

(fn `EndCombo`)

(fn `OffCollision`
  (`KismetArrayLibrary.Array_Clear` (`self.HittedActors`)))

(fn `OnCollision`
  (params (CollisionType :type "/Game/Enums/ECollisionType Enum" :default "NewEnumerator0")))

(fn `PlayComboMontage`
  (bind (_output_type _output_montage _output_playrate _output_startsection _output_bcanmove) (break `/Game/Structs/FMelee` (`|GetArrayItem` (`self.MeleeDatas`) (`self.ComboCount`))))
  (bind _ascharacter (cast `Character` (`self.GetOwner`)))
  (`Character.PlayAnimMontage` _ascharacter _output_montage _output_playrate _output_startsection)
  (`self.SetMove` _output_bcanmove))

(fn `SendDamage`
  (params (OtherActor :type "Actor Object Reference") (Damage :type "Float (double-precision)"))
  (returns (Result :type Boolean))
  (locals (bEverHitted :type Boolean))
  (for _array_element (`self.HittedActors`)
    (if (== _array_element (`local.OtherActor`))
      (set `local.bEverHitted` true)
      (break)))
  (if (not (`local.bEverHitted`))
    (`KismetArrayLibrary.Array_Add` (`self.HittedActors`) (`local.OtherActor`))
    (bind _result (`parent.SendDamage` (`local.OtherActor`) (`local.Damage`)))
    (return _result)))

(fn `StartCombo`)

(fn `UserConstructionScript`
  (`parent.UserConstructionScript`))