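; BP_Skill_Throw is a magic skill that lets a character throw a selectable item from the hand.
; Equipping shows the current item's attach particle and turns on player aiming, and unequipping reverses both.
; Spell plays a fireball montage, while a separate DoThrow event spawns the item's class at the Hand_Throw socket along the control rotation.
; SetCurrentItemIndex picks the ThrowItems entry by class and updates the particle.
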(event `self.ReceiveBeginPlay`
  (bind (_output_throwitemclass _output_attachparticle) (break `/Game/Structs/FThrowItem` (`|GetArrayItem` (`self.ThrowItems`) (`self.CurrentItemIndex`))))
  (`parent.ReceiveBeginPlay`)
  (`ParticleSystemComponent.SetTemplate` (`self.AttachParticle`) _output_attachparticle)
  (`SceneComponent.SetVisibility` (`self.AttachParticle`) false false))

(event `self.OnEquip`
  (`parent.OnEquip`)
  (`SceneComponent.SetVisibility` (`self.AttachParticle`) true false)
  (bind _asbp_player (cast `/Game/Player/BP_Player` (`self.GetOwnerToCharacter`)))
  (`/Game/Player/BP_Player.OnAim` _asbp_player))

(event `self.OnUnequip`
  (`parent.OnUnequip`)
  (`SceneComponent.SetVisibility` (`self.AttachParticle`) false false)
  (bind _asbp_player (cast `/Game/Player/BP_Player` (`self.GetOwnerToCharacter`)))
  (`/Game/Player/BP_Player.OffAim` _asbp_player))

(event `self.Spell`
  (`parent.Spell`)
  (`Character.PlayAnimMontage` (`self.GetOwnerToCharacter`) "/Game/Character/Animations/Magic/MG_Fireball_03_Montage.MG_Fireball_03_Montage" 1.0 "None"))

(event `DoThrow`
  (bind _output_throwitemclass (break `/Game/Structs/FThrowItem` (`|GetArrayItem` (`self.ThrowItems`) (`self.CurrentItemIndex`))))
  (`|SpawnActorFromClass` _output_throwitemclass (`KismetMathLibrary.MakeTransform` (`SceneComponent.GetSocketLocation` (`Character.Mesh` (`self.GetOwnerToCharacter`)) "Hand_Throw") (`Controller.GetControlRotation` (`GameplayStatics.GetPlayerController` 0)) (`self.ParticleScale`)) "Undefined" "OverrideRootScale" self null))

(event `self.EndSpell`
  (`parent.EndSpell`))

(fn `SetCurrentItemIndex`
  (params (NewItemClass :type "/Game/Weapons/Magic/BP_ThrowItem Class Reference"))
  (locals (Iterator :type Integer))
  (bind _output_throwitemclass (break `/Game/Structs/FThrowItem` (`|GetArrayItem` (`self.ThrowItems`) (`local.Iterator`))))
  (bind (_output_throwitemclass_2 _output_attachparticle) (break `/Game/Structs/FThrowItem` (`|GetArrayItem` (`self.ThrowItems`) (`self.CurrentItemIndex`))))
  (for (_ _array_index) (`self.ThrowItems`)
    (set `local.Iterator` _array_index)
    (if (== (`local.NewItemClass`) _output_throwitemclass)
      (break)))
  (set `self.CurrentItemIndex` (`local.Iterator`))
  (`ParticleSystemComponent.SetTemplate` (`self.AttachParticle`) _output_attachparticle))

(fn `UserConstructionScript`
  (`parent.UserConstructionScript`))