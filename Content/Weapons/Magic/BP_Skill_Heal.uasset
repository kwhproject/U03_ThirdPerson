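; Heal skill Blueprint that restores a fixed amount of health to the character casting it.
; It extends a parent skill's Spell event to lock movement through the owner's magic interface or object and play a buff montage.
; Health is added immediately through the owner's StatusComponent, if valid, and the new value is debug-printed.
; EndSpell calls the parent and re-enables movement.
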(event `self.Spell`
  (bind _ascharacter (`self.GetOwnerToCharacter`))
  (bind _returnvalue (`self.GetComponentByClass` _ascharacter "/Game/Components/StatusComponent.StatusComponent_C"))
  (`parent.Spell`)
  (`/Game/Weapons/BP_Weapon.SetMove` (`self.Get Owner To Magic`) false)
  (`Character.PlayAnimMontage` _ascharacter "/Game/Character/Animations/Magic/MG_Buff_Montage.MG_Buff_Montage" 1.0 "None")
  (`/Engine/EditorBlueprintResources/StandardMacros.IsValid` _returnvalue
    (:`Is Valid`
      (`/Game/Components/StatusComponent.IncreaseHealth` _returnvalue 10.0)
      (`KismetSystemLibrary.PrintString` (`KismetStringLibrary.Conv_DoubleToString` (`/Game/Components/StatusComponent.CurrentHealth` _returnvalue))))))

(event `self.EndSpell`
  (`parent.EndSpell`)
  (`/Game/Weapons/BP_Weapon.SetMove` (`self.Get Owner To Magic`) true))

(fn `UserConstructionScript`
  (`parent.UserConstructionScript`))