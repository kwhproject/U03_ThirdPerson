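; BP_ThrowItem is a thrown magic item, apparently a base class, that expires ten seconds after spawning.
; PlayHitParticle activates a given particle on a hit BP_Enemy's HitEffect component, disables its own collision, hides, then stops the effect and destroys itself after a short delay.
; Helpers walk the owner chain to BP_Skill_Throw and BP_Magic.
; BeginOverlap is an empty stub taking impact and damage parameters.
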(event `self.ReceiveBeginPlay`
  (`self.SetLifeSpan` 10.0))

(event `PlayHitParticle`
  (params (OtherActor :type "Actor Object Reference") (EmberParticle :type "ParticleSystem Object Reference"))
  (bind _asbp_enemy (cast `/Game/Enemys/BP_Enemy` OtherActor))
  (bind _output_get (set `self.ParticleComp` (`/Game/Enemys/BP_Enemy.HitEffect` _asbp_enemy)))
  (`ParticleSystemComponent.SetTemplate` _output_get EmberParticle)
  (`ActorComponent.SetActive` (`self.ParticleComp`) true false)
  (`PrimitiveComponent.SetCollisionEnabled` (`self.Sphere`) "NoCollision")
  (`self.SetActorHiddenInGame` true)
  (`KismetSystemLibrary.Delay` 2.0)
  (`ActorComponent.SetActive` (`self.ParticleComp`) false false)
  (`self.K2_DestroyActor`))

(fn `Begin Overlap`
  (params (`Other Actor` :type "Actor Object Reference") (ImpactParticle :type "ParticleSystem Object Reference") (ImpactLocation :type "Vector Structure") (ImpactScale :type "Vector Structure" :default (1.0 1.0 1.0)) (Damage :type "Float (double-precision)" :default 1.0)))

(fn `Get Owner to Magic`
  (returns (`As BP Magic` :type "/Game/Weapons/Magic/BP_Magic Object Reference"))
  (bind _asbp_magic (cast `/Game/Weapons/Magic/BP_Magic` (`self.GetOwner` (`self.Get Owner to Throw`))))
  (return _asbp_magic))

(fn `Get Owner to Throw`
  (returns (`As BP Skill Throw` :type "/Game/Weapons/Magic/BP_Skill_Throw Object Reference"))
  (bind _asbp_skill_throw (cast `/Game/Weapons/Magic/BP_Skill_Throw` (`self.GetOwner`)))
  (return _asbp_skill_throw))

(fn `UserConstructionScript`)