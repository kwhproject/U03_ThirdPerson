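; BP_ThunderBall is a magic projectile that damages what it hits and then destroys itself.
; On sphere overlap it reads single damage from its DamageComponent and calls BeginOverlap, which spawns a thunder ball hit particle at its location.
; The particle is rotated along the line from the magic owner's owning actor toward the hit actor, and damage is routed through the owning magic's SendDamage.
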(event `self.Sphere.OnComponentBeginOverlap`
  (params (OverlappedComponent :type "PrimitiveComponent Object Reference") (OtherActor :type "Actor Object Reference") (OtherComp :type "PrimitiveComponent Object Reference") (OtherBodyIndex :type Integer) (bFromSweep :type Boolean) (SweepResult :type "HitResult Structure (by ref)"))
  (bind _returnvalue (`/Game/Components/DamageComponent.GetSingleDamage` (`self.DamageComponent`)))
  (`self.Begin Overlap` OtherActor "/Game/FXVarietyPack/Particles/P_ky_ThunderBallHit.P_ky_ThunderBallHit" (0.0 0.0 0.0) (0.25 0.25 0.25) _returnvalue)
  (`self.K2_DestroyActor`))

(fn `Begin Overlap`
  (params (`Other Actor` :type "Actor Object Reference") (ImpactParticle :type "ParticleSystem Object Reference") (ImpactLocation :type "Vector Structure") (ImpactScale :type "Vector Structure") (Damage :type "Float (double-precision)"))
  (`|ExecutionSequence`
    (:`then_0`
      (`GameplayStatics.SpawnEmitterAtLocation` (`local.ImpactParticle`) (+ (`self.K2_GetActorLocation`) (`local.ImpactLocation`)) (`KismetMathLibrary.FindLookAtRotation` (`self.K2_GetActorLocation` (`self.GetOwner` (`self.Get Owner to Magic`))) (`self.K2_GetActorLocation` (`local.Other Actor`))) (`local.ImpactScale`)))
    (:`then_1`
      (`/Game/Weapons/BP_Weapon.SendDamage` (`self.Get Owner to Magic`) (`local.Other Actor`) (`local.Damage`)))))

(fn `UserConstructionScript`
  (`parent.UserConstructionScript`))