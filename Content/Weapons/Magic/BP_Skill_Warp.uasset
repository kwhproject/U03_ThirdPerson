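; Magic skill Blueprint that teleports its owning character to the point under the mouse cursor.
; While equipped, Tick traces WorldStatic under the cursor and places a targeting decal aligned to the hit normal, hiding it otherwise.
; Spell stores the hit, locks movement and plays the warp montage, or ends the attack without a hit.
; DoWarp moves the owner there with sweep, raised by capsule half-height; EndSpell restores movement.
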(event `self.ReceiveBeginPlay`
  (`SceneComponent.SetVisibility` (`self.Decal`) false false))

(event `self.OnEquip`
  (`parent.OnEquip`)
  (set `self.bEquipThis` true))

(event `self.OnUnequip`
  (`parent.OnUnequip`)
  (set `self.bEquipThis` false))

(event `self.ReceiveTick`
  (params (DeltaSeconds :type "Float (single-precision)"))
  (if (`self.bEquipThis`)
    (bind (_location _impactnormal) (`self.GetCursorTransform`)
      (:`True`
        (`SceneComponent.K2_SetWorldLocation` (`self.Decal`) _location false false)
        (`SceneComponent.K2_SetWorldRotation` (`self.Decal`) (`KismetMathLibrary.Conv_VectorToRotator` _impactnormal) false false)
        (`SceneComponent.SetVisibility` (`self.Decal`) true false))
      (:`False`
        (`SceneComponent.SetVisibility` (`self.Decal`) false false :!label _label)))
    (else
      (goto _label))))

(event `self.Spell`
  (`parent.Spell`)
  (bind _location (`self.GetCursorTransform`)
    (:`True`
      (set `self.WarpPoint` _location)
      (set `self.bCanWarp` true)
      (`/Game/Weapons/BP_Weapon.SetMove` (`self.Get Owner To Magic`) false)
      (`Character.PlayAnimMontage` (`self.GetOwnerToCharacter`) "/Game/Character/Animations/Magic/MG_Warp_Montage.MG_Warp_Montage" 2.0 "None"))
    (:`False`
      (`/Game/Weapons/BP_Weapon.EndAttack` (`self.Get Owner To Magic`))
      (set `self.bCanWarp` false))))

(event `DoWarp`
  (bind (_warppoint_x _warppoint_y _warppoint_z) (`KismetMathLibrary.BreakVector` (`self.WarpPoint`)))
  (if (`self.bCanWarp`)
    (set `self.bCanWarp` false)
    (`self.K2_SetActorLocation` (`self.GetOwnerToCharacter`) (`KismetMathLibrary.MakeVector` _warppoint_x _warppoint_y (+ _warppoint_z (`CapsuleComponent.GetScaledCapsuleHalfHeight` (`Character.CapsuleComponent` (`self.GetOwnerToCharacter`))))) true false)))

(event `self.EndSpell`
  (`parent.EndSpell`)
  (`/Game/Weapons/BP_Weapon.SetMove` (`self.Get Owner To Magic`) true))

(fn `UserConstructionScript`
  (`parent.UserConstructionScript`))