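; BP_Skill appears to be a base for magic skills, owned by a BP_Magic weapon.
; It exposes Spell, EndSpell, OnEquip and OnUnequip events, all empty except OnEquip, which calls SetMove(true) on the owning magic.
; Helper functions resolve the ownership chain, casting the skill's owner to BP_Magic and that magic's owner to Character.
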(event `Spell`)

(event `EndSpell`)

(event `OnEquip`
  (`/Game/Weapons/BP_Weapon.SetMove` (`self.Get Owner To Magic`) true))

(event `OnUnequip`)

(fn `Get Owner To Magic`
  (returns (`AsBP Magic` :type "/Game/Weapons/Magic/BP_Magic Object Reference"))
  (bind _asbp_magic (cast `/Game/Weapons/Magic/BP_Magic` (`self.GetOwner`)))
  (return _asbp_magic))

(fn `GetOwnerToCharacter`
  (returns (AsCharacter :type "Character Object Reference"))
  (bind _ascharacter (cast `Character` (`self.GetOwner` (`self.Get Owner To Magic`))))
  (return _ascharacter))

(fn `UserConstructionScript`)