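; BP_Enemy is a melee enemy character that spawns a holstered greatsword and displays its name and health.
; AnyDamage lowers StatusComponent health, updates the HP widget, plays a hit montage, turns it toward the attacker and flashes dynamic body materials red.
; On death it ragdolls away from the attacker with damage-scaled force, then destroys itself and the sword after a delay.
; Combat state and weapon functions are partly stubbed, including attach, movement and spellcasting.
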(event `self.ReceiveBeginPlay`
  (`|ExecutionSequence`
    (:`then_0`
      (bind _returnvalue (`|SpawnActorFromClass` "/Game/Weapons/Melee/BP_GreatSword.BP_GreatSword_C" (`KismetMathLibrary.MakeTransform` (0.0 0.0 0.0)) "Undefined" "OverrideRootScale" self null))
      (bind _output_get (set `self.GreatSword` _returnvalue))
      (`self.K2_AttachToComponent` _output_get (`self.Mesh`) "Holster_GreatSword" "KeepRelative" "KeepRelative" "KeepRelative" true))
    (:`then_1`
      (`TextRenderComponent.K2_SetText` (`self.CharacterName`) (`KismetTextLibrary.Conv_StringToText` (`KismetSystemLibrary.GetDisplayName` self))))
    (:`then_2`
      (`self.UpdateHealth`))))

(event `self.ReceiveAnyDamage`
  (params (Damage :type "Float (single-precision)") (DamageType :type "DamageType Object Reference") (InstigatedBy :type "Controller Object Reference") (DamageCauser :type "Actor Object Reference"))
  (set `self.Causer` DamageCauser)
  (bind _ascharacter (cast `Character` (`Controller.K2_GetPawn` InstigatedBy)))
  (set `self.Attacker` _ascharacter)
  (bind _output_get (set `self.Damage` Damage))
  (`/Game/Components/StatusComponent.DecreaseHealth` (`self.StatusComponent`) _output_get)
  (`self.UpdateHealth`)
  (set `self.StateType` "NewEnumerator8")
  (`self.PlayAnimMontage` "/Game/Character/Animations/Common/HitReaction_Montage.HitReaction_Montage" 3.0)
  (`self.K2_SetActorRotation` (`KismetMathLibrary.FindLookAtRotation` (`self.K2_GetActorLocation`) (`self.K2_GetActorLocation` (`self.Attacker`))))
  (`self.ChangeBodyColor` (struct :`R` 1.0 :`A` 1.0))
  (`KismetSystemLibrary.Delay` 0.1)
  (`self.ChangeBodyColor` (`self.BodyColor`))
  (if (`/Game/Components/StatusComponent.IsDead` (`self.StatusComponent`))
    (if (`|EnumInequality` (`self.StateType`) "NewEnumerator4")
      (set `self.StateType` "NewEnumerator4")
      (`self.Ragdoll`)
      (`KismetSystemLibrary.Delay` 5.0)
      (`self.Dead`))))

(event `Dead`
  (`self.K2_DestroyActor` (`self.GreatSword`))
  (`self.K2_DestroyActor`))

(fn `Attach`)

(fn `AttachWeapon`
  (returns (Result :type Boolean))
  (`self.Attach`)
  (return false))

(fn `ChangeBodyColor`
  (params (NewColor :type "LinearColor Structure"))
  (for _array_element (`self.DynamicMaterials`)
    (`MaterialInstanceDynamic.SetVectorParameterValue` _array_element "BodyColor" (`local.NewColor`))))

(fn `CreateDynamicMaterial`
  (`|ExecutionSequence`
    (:`then_0`
      (bind _returnvalue (`KismetMaterialLibrary.CreateDynamicMaterialInstance` "/Game/Character/Materials/M_UE4Man_Body_Inst.M_UE4Man_Body_Inst"))
      (`KismetArrayLibrary.Array_Add` (`self.DynamicMaterials`) _returnvalue))
    (:`then_1`
      (bind _returnvalue_2 (`KismetMaterialLibrary.CreateDynamicMaterialInstance` "/Game/Character/Materials/M_UE4Man_ChestLogo.M_UE4Man_ChestLogo"))
      (`KismetArrayLibrary.Array_Add` (`self.DynamicMaterials`) _returnvalue_2))
    (:`then_2`
      (`PrimitiveComponent.SetMaterial` (`self.Mesh`) 0 (`|GetArrayItem` (`self.DynamicMaterials`)))
      (`PrimitiveComponent.SetMaterial` (`self.Mesh`) 1 (`|GetArrayItem` (`self.DynamicMaterials`) 1)))))

(fn `Detach`)

(fn `DetachWeapon`
  (returns (Result :type Boolean))
  (`self.Detach`)
  (return false))

(fn `Equipped`
  (set `self.StateType` "NewEnumerator0"))

(fn `EquippedWeapon`
  (returns (Return :type Boolean))
  (`self.Equipped`)
  (return false))

(fn `GetCombatType`
  (returns (CombatType :type "/Game/Enums/ECombatType Enum"))
  (return (`self.CombatType`)))

(fn `GetCurrentWeapon`
  (returns (CurrentWeapon :type "/Game/Weapons/BP_Weapon Object Reference"))
  (return (`self.CurrentWeapon`)))

(fn `IsStateAttacking`
  (returns (Result :type Boolean))
  (return (`|EnumEquality` (`self.StateType`) "NewEnumerator3")))

(fn `IsStateIdling`
  (returns (Result :type Boolean))
  (return (`|EnumEquality` (`self.StateType`) "NewEnumerator0")))

(fn `Ragdoll`
  (`PrimitiveComponent.SetCollisionEnabled` (`self.CapsuleComponent`) "NoCollision")
  (set `SkeletalMeshComponent.GlobalAnimRateScale` 0.0 (`self.Mesh`))
  (`PrimitiveComponent.SetSimulatePhysics` (`self.Mesh`) true)
  (`PrimitiveComponent.SetCollisionEnabled` (`self.Mesh`) "QueryAndPhysics")
  (`PrimitiveComponent.AddForce` (`self.Mesh`) (* (* (`KismetMathLibrary.GetDirectionUnitVector` (`self.K2_GetActorLocation` (`self.Attacker`)) (`self.K2_GetActorLocation`)) (`self.Damage`)) 250000.0) "None" false))

(fn `SetCurrentWeapon`
  (params (NewWeapon :type "/Game/Weapons/BP_Weapon Object Reference"))
  (returns (Result :type Boolean))
  (`/Engine/EditorBlueprintResources/StandardMacros.IsValid` (`self.CurrentWeapon`)
    (:`Is Valid`
      (`/Game/Weapons/BP_Weapon.OnUnequip` (`self.CurrentWeapon`)))
    (:`Is Not Valid`
      _))
  (`/Engine/EditorBlueprintResources/StandardMacros.IsValid` (`local.NewWeapon`)
    (:`Is Valid`
      (bind _output_get (set `self.CurrentWeapon` (`local.NewWeapon`)))
      (`/Game/Weapons/BP_Weapon.OnEquip` _output_get))
    (:`Is Not Valid`
      (set `self.CurrentWeapon` null)))
  (return false))

(fn `SetMove`
  (params (NewMove :type Boolean))
  (returns (Result :type Boolean))
  (return false))

(fn `SetStateAttacking`
  (returns (Result :type Boolean))
  (set `self.StateType` "NewEnumerator3")
  (return false))

(fn `SetStateHitted`
  (returns (Result :type Boolean))
  (set `self.StateType` "NewEnumerator0")
  (return false))

(fn `SetStateIdling`
  (returns (Result :type Boolean))
  (set `self.StateType` "NewEnumerator0")
  (return false))

(fn `SetStateSpelling`
  (returns (Result :type Boolean))
  (`KismetSystemLibrary.PrintString` "마법 미개발")
  (return false))

(fn `Unequipped`
  (set `self.StateType` "NewEnumerator0"))

(fn `UnequippedWeapon`
  (returns (Result :type Boolean))
  (`self.Unequipped`)
  (return false))

(fn `UpdateHealth`
  (bind _statuscomponent (`self.StatusComponent`))
  (bind _aswb_enemy_hp (cast `/Game/Widgets/WB_EnemyHP` (`WidgetComponent.GetUserWidgetObject` (`self.HealthWidget`))))
  (`/Game/Widgets/WB_EnemyHP.UpdateHealth` _aswb_enemy_hp (`/Game/Components/StatusComponent.CurrentHealth` _statuscomponent) (`/Game/Components/StatusComponent.MaxHealth` _statuscomponent)))

(fn `UserConstructionScript`
  (`self.CreateDynamicMaterial`)
  (`self.ChangeBodyColor` (`self.BodyColor`)))